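; CoffeeCup_BP is a player-controlled physics body that flies with six degrees of freedom and collects items for score.
; Input axes apply thrust and torque impulses along the Cube's local axes, with an invert toggle for pitch.
; Tick adds velocity-dependent linear and angular drag, only the linear part scaled by delta time.
; Any overlapped actor is destroyed and increments the CoffeCupGameMode_BP score; Fire only prints.
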(event `self.ReceiveActorBeginOverlap`
  (params (OtherActor :type "Actor Object Reference"))
  ;[1 1 1] Get Collectible and Increase Score
  (`self.K2_DestroyActor` OtherActor)
  (bind _ascoffe_cup_game_mode_bp (cast `/Game/Blueprints/CoffeCupGameMode_BP` (`GameplayStatics.GetGameMode`)))
  (set `/Game/Blueprints/CoffeCupGameMode_BP.score` (+ (`/Game/Blueprints/CoffeCupGameMode_BP.score` _ascoffe_cup_game_mode_bp) 1) _ascoffe_cup_game_mode_bp))

(event `InputAction|Fire`
  (params (Key :type "Key Structure"))
  (:`Pressed`
    (`KismetSystemLibrary.PrintString` "Fire_THRUST")))

(event `self.ReceiveTick`
  (params (DeltaSeconds :type "Float (single-precision)"))
  (bind _cube (`self.Cube`))
  (bind _returnvalue (`SceneComponent.GetComponentVelocity` _cube))
  (bind _returnvalue_2 (`PrimitiveComponent.GetPhysicsAngularVelocityInDegrees` _cube "None"))
  (`PrimitiveComponent.AddImpulse` _cube (* (* _returnvalue (* DeltaSeconds -1e-05)) (`KismetMathLibrary.Square` (`KismetMathLibrary.VSize` _returnvalue))) "None" true)
  (`PrimitiveComponent.AddAngularImpulseInDegrees` _cube (* (* _returnvalue_2 -0.001) (`KismetMathLibrary.VSize` _returnvalue_2)) "None" true))

(event `self.ReceiveBeginPlay`
  ;[1 1 1] Spawn Multiple Players
  (`KismetSystemLibrary.PrintString` "SOPANWING"))

(event `InputAxis|Roll`
  (params (AxisValue :type "Float (single-precision)"))
  (bind _cube (`self.Cube`))
  ;[1 1 1] Torque Up/Down - Roll
  (`PrimitiveComponent.AddAngularImpulseInRadians` _cube (* (`SceneComponent.GetForwardVector` _cube) (* AxisValue (* -1 (`self.Rotation_Multiplier`)))) "None" true))

(event `InputAxis|IncreaseThrottle`
  (params (AxisValue :type "Float (single-precision)"))
  (bind _cube (`self.Cube`))
  ;[1 1 1] Thrust Forward/Backward
  (`PrimitiveComponent.AddImpulse` _cube (* (`SceneComponent.GetForwardVector` _cube) (* AxisValue (`self.Speed_Multiplier`))) "None" true))

(event `InputAxis|MoveRight`
  (params (AxisValue :type "Float (single-precision)"))
  (bind _cube (`self.Cube`))
  ;[1 1 1] Thrust Left/Right
  (`PrimitiveComponent.AddImpulse` _cube (* (`SceneComponent.GetRightVector` _cube) (* AxisValue (`self.Speed_Multiplier`))) "None" true))

(event `InputAxis|Yaw`
  (params (AxisValue :type "Float (single-precision)"))
  (bind _cube (`self.Cube`))
  ;[1 1 1] Torque Left/Right - Yaw
  (`PrimitiveComponent.AddAngularImpulseInRadians` _cube (* (`SceneComponent.GetUpVector` _cube) (* AxisValue (* 1 (`self.Rotation_Multiplier`)))) "None" true))

(event `InputAxis|Pitch`
  (params (AxisValue :type "Float (single-precision)"))
  (bind _cube (`self.Cube`))
  ;[1 1 1] Torque Left/Right - Pitch
  (`PrimitiveComponent.AddAngularImpulseInRadians` _cube (* (`SceneComponent.GetRightVector` _cube) (* AxisValue (* (`self.Pitch_Inversion`) (`self.Rotation_Multiplier`)))) "None" true))

(event `InputAxis|MoveUp`
  (params (AxisValue :type "Float (single-precision)"))
  (bind _cube (`self.Cube`))
  ;[1 1 1] Thrust Up/Down
  (`PrimitiveComponent.AddImpulse` _cube (* (`SceneComponent.GetUpVector` _cube) (* AxisValue (`self.Speed_Multiplier`))) "None" true))

(event `InputAction|Invert`
  (params (Key :type "Key Structure"))
  ;[1 1 1] Y to invert (pitch)
  (:`Pressed`
    (set `self.Pitch_Inversion` (* (`self.Pitch_Inversion`) -1))))

(fn `UserConstructionScript`)