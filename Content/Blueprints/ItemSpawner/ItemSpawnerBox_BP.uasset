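; Item spawner box that scatters a batch of Collectibles_BP actors within its ItemSpawnBounds component on BeginPlay.
; SpawnNewItem picks a random point from the bounds, though the Y maximum adds the origin to itself instead of the box extent.
; A small sphere overlap rejects points touching ItemLessSphere_BP actors, making those exclusion zones.
; Rejected points trigger a recursive retry with no attempt limit.
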(event `self.ReceiveBeginPlay`
  (for _ (range 51)
    (`self.SpawnNewItem`)))

(event `SpawnNewItem`
  (bind (_origin _boxextent) (`KismetSystemLibrary.GetComponentBounds` (`self.ItemSpawnBounds`)))
  (bind _x (.x _origin))
  (bind _y (.y _origin))
  (bind _z (.z _origin))
  (bind _x_2 (.x _boxextent))
  (bind _z_2 (.z _boxextent))
  (set `self.randomLocation` (`KismetMathLibrary.MakeVector` (`KismetMathLibrary.RandomFloatInRange` (- _x _x_2) (+ _x _x_2)) (`KismetMathLibrary.RandomFloatInRange` (- _y (.y _boxextent)) (+ _y _y)) (`KismetMathLibrary.RandomFloatInRange` (- _z _z_2) (+ _z _z_2))))
  (bind (_outactors _returnvalue) (`KismetSystemLibrary.SphereOverlapActors` (`self.randomLocation`) 0.5 (`|MakeArray` "ObjectTypeQuery2" :!type "EObjectTypeQuery Enum") "/Game/Blueprints/ItemSpawner/ItemLessSphere_BP.ItemLessSphere_BP_C"))
  (if _returnvalue
    (`self.SpawnNewItem`)
    (else
      (`|SpawnActorFromClass` "/Game/Blueprints/ItemSpawner/Collectibles_BP.Collectibles_BP_C" (`KismetMathLibrary.Conv_VectorToTransform` (`self.randomLocation`)) "Undefined" "OverrideRootScale" null null))))

(fn `UserConstructionScript`)